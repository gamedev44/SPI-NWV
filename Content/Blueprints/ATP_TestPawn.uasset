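; ATP_TestPawn is a test pawn for async tick physics functions, with mouse look input.
; Each AsyncTick wakes the static mesh's bodies and applies a random impulse through ATPAddImpulse.
; It also prints the skeletal mesh's bone velocity magnitude from the game API beside the ATP physics API result, flagging whether they differ.
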(event `self.AsyncTick`
  (params (DeltaTime :type "Float (single-precision)"))
  (bind _skeletalmesh (`self.SkeletalMesh`))
  (bind _returnvalue (`SkinnedMeshComponent.GetBoneName` _skeletalmesh 4))
  (`PrimitiveComponent.WakeAllRigidBodies` (`self.StaticMesh`))
  (bind _returnvalue_2 (`PrimitiveComponent.GetPhysicsLinearVelocityAtPoint` _skeletalmesh (0.0 0.0 0.0) _returnvalue))
  (bind _returnvalue_3 (`AsyncTickFunctions.ATP_GetLinearVelocityAtPoint` _skeletalmesh (0.0 0.0 0.0) _returnvalue))
  (bind _returnvalue_4 (`KismetMathLibrary.VSize` _returnvalue_2))
  (bind _returnvalue_5 (`KismetMathLibrary.VSize` _returnvalue_3))
  (`KismetSystemLibrary.PrintString` (`KismetTextLibrary.Conv_TextToString` (`|FormatText` "Game API: {0} \nPhysics API: {1} \nNOT_EQUAL: {2} " _returnvalue_4 _returnvalue_5 (!= _returnvalue_4 _returnvalue_5))) true true (struct :`G` 0.66 :`B` 1.0 :`A` 1.0) 2.0 "LINEAR_VELOCITY")
  (`AsyncTickFunctions.ATP_AddImpulse` (`self.StaticMesh`) (* (`KismetMathLibrary.RandomUnitVector`) (`KismetMathLibrary.RandomFloatInRange` 5.0 500.0))))

(event `InputAxis|Look Up / Down Mouse`
  (params (AxisValue :type "Float (single-precision)"))
  (`self.AddControllerPitchInput` AxisValue))

(event `InputAxis|Turn Right / Left Mouse`
  (params (AxisValue :type "Float (single-precision)"))
  (`self.AddControllerYawInput` AxisValue))

(fn `UserConstructionScript`)