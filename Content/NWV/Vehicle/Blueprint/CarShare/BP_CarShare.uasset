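; Car share station that lets the player pick a car from DT_Cars and drive off in it.
; On BeginPlay or when a vehicle enters the trigger, it shows a preview dummy car and name widget; an entering vehicle is destroyed and the station possessed.
; A/D step through the table rows, reloading the dummy's config.
; Enter spawns and possesses the configured vehicle at NewCarSpawnPoint, or at a randomized transform if unset.
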(event `self.ReceiveBeginPlay`
  ;[1 1 1] game start enter
  (bind _outrownames (`DataTableFunctionLibrary.GetDataTableRowNames` "/Game/NWV/Vehicle/Data/DT_Cars.DT_Cars"))
  (set `self.CarNames` _outrownames)
  (set `self.PlayerController` (`GameplayStatics.GetPlayerController` 0))
  ;[1 1 1] reset selected car
  (set `self.Name` (`|GetArrayItem` (`self.CarNames`)) :!label _label)
  (set `self.CarIndex` 0)
  (`/Engine/EditorBlueprintResources/StandardMacros.IsValid` (`self.DummyCar`)
    (:`Is Valid`
      (bind _returnvalue (`|GetDataTableRow` "/Game/NWV/Vehicle/Data/DT_Cars.DT_Cars" (`self.Name`))
        (:`then`
          (bind _output_get (set `self.Car Config` _returnvalue))
          (`/Game/NWV/Vehicle/Blueprint/CarShare/BP_DummyCar.Load Config` (`self.DummyCar`) _output_get))))
    (:`Is Not Valid`
      (bind _returnvalue_2 (`|SpawnActorFromClass` "/Game/NWV/Vehicle/Blueprint/CarShare/BP_DummyCar.BP_DummyCar_C" (`KismetMathLibrary.MakeTransform` (+ (.location (`self.GetTransform`)) (0.0 0.0 30.0)) (.rotation (`self.GetTransform`))) "AlwaysSpawn" "MultiplyWithRoot" null null))
      (bind _output_get_2 (set `self.DummyCar` _returnvalue_2))
      (bind _returnvalue_3 (`|GetDataTableRow` "/Game/NWV/Vehicle/Data/DT_Cars.DT_Cars" (`self.Name`))
        (:`then`
          (bind _output_get_3 (set `self.Car Config` _returnvalue_3))
          (`/Game/NWV/Vehicle/Blueprint/CarShare/BP_DummyCar.Load Config` _output_get_2 _output_get_3)))))
  (`/Engine/EditorBlueprintResources/StandardMacros.IsValid` (`self.WidgetCarShare`)
    (:`Is Valid`
      (`UserWidget.AddToViewport` (`self.WidgetCarShare`) 0))
    (:`Is Not Valid`
      (bind _returnvalue_4 (`|CreateWidget` "/Game/NWV/Vehicle/Widget/Widget_CarShare.Widget_CarShare_C" (`self.PlayerController`)))
      (bind _output_get_4 (set `self.WidgetCarShare` _returnvalue_4))
      (set `/Game/NWV/Vehicle/Widget/Widget_CarShare.CarShare` self (`self.WidgetCarShare`))
      (`UserWidget.AddToViewport` _output_get_4 0)))
  (`/Game/NWV/Vehicle/Widget/Widget_CarShare.Set Car Name Text` (`self.WidgetCarShare`) (`self.Name`))
  (`WidgetBlueprintLibrary.SetInputMode_GameOnly` (`self.PlayerController`)))

(event `self.EntryTrigger.OnComponentBeginOverlap`
  (params (OverlappedComponent :type "PrimitiveComponent Object Reference") (OtherActor :type "Actor Object Reference") (OtherComp :type "PrimitiveComponent Object Reference") (OtherBodyIndex :type Integer) (bFromSweep :type Boolean) (SweepResult :type "HitResult Structure (by ref)"))
  ;[1 1 1] enter with car
  (bind _asprt_nwheel_vehicle (cast `/Game/NWV/Vehicle/Blueprint/PRT_NWheelVehicle` OtherActor))
  (bind _output_get (set `self.Car` _asprt_nwheel_vehicle))
  (`/Game/NWV/Vehicle/Blueprint/PRT_NWheelVehicle.RemoveCarHud` _output_get)
  (bind _output_get_2 (set `self.PlayerController` (`GameplayStatics.GetPlayerController` 0)))
  (`Controller.UnPossess` _output_get_2)
  (`self.K2_DestroyActor` (`self.Car`))
  (`Controller.Possess` (`self.PlayerController`) self)
  (goto _label))

(event `Key|D`
  (params (Key :type "Key Structure"))
  (bind _widgetcarshare (`self.WidgetCarShare`))
  (:`Pressed`
    (if (< (`self.CarIndex`) (`KismetArrayLibrary.Array_LastIndex` (`self.CarNames`)))
      (`/Engine/EditorBlueprintResources/StandardMacros.IncrementInt` (`self.CarIndex`)
        (:`  `
          (bind _output_get (set `self.Name` (`|GetArrayItem` (`self.CarNames`) (`self.CarIndex`)) :!label _label_2))
          (bind _returnvalue (`|GetDataTableRow` "/Game/NWV/Vehicle/Data/DT_Cars.DT_Cars" _output_get)
            (:`then`
              (`self.ChangeDummyCar` _returnvalue)
              (`/Engine/EditorBlueprintResources/StandardMacros.IsValid` _widgetcarshare
                (:`Is Valid`
                  (`/Game/NWV/Vehicle/Widget/Widget_CarShare.Set Car Name Text` _widgetcarshare (`self.Name`)))))))))))

(event `Key|A`
  (params (Key :type "Key Structure"))
  (:`Pressed`
    (if (> (`self.CarIndex`) 0)
      (`/Engine/EditorBlueprintResources/StandardMacros.DecrementInt` (`self.CarIndex`)
        (:`  `
          (goto _label_2))))))

(event `Key|Enter`
  (params (Key :type "Key Structure"))
  (:`Pressed`
    (`self.LetsRide`)))

(fn `ChangeDummyCar`
  (params (CarConfig :type "/Game/NWV/Vehicle/CustomType/Config/CarConfig Structure"))
  (bind _dummycar (`self.DummyCar`))
  (set `self.Car Config` CarConfig)
  (`/Engine/EditorBlueprintResources/StandardMacros.IsValid` _dummycar
    (:`Is Valid`
      (`/Game/NWV/Vehicle/Blueprint/CarShare/BP_DummyCar.Load Config` _dummycar (`self.Car Config`)))))

(fn `LetsRide`
  (locals (Tr :type "Transform Structure"))
  (bind _newcarspawnpoint (`self.NewCarSpawnPoint`))
  (bind _playercontroller (`self.PlayerController`))
  (`/Engine/EditorBlueprintResources/StandardMacros.IsValid` (`self.Car`)
    (:`Is Valid`
      (`self.K2_DestroyActor` (`self.Car`)))
    (:`Is Not Valid`
      _))
  (`/Engine/EditorBlueprintResources/StandardMacros.IsValid` _newcarspawnpoint
    (:`Is Valid`
      (set `local.Tr` (`self.GetTransform` _newcarspawnpoint)))
    (:`Is Not Valid`
      (set `local.Tr` (`KismetMathLibrary.MakeTransform` (* (`KismetMathLibrary.RotateAngleAxis` (`KismetMathLibrary.GetForwardVector` (.rotation (`self.GetTransform`))) (`KismetMathLibrary.RandomFloatInRange` -180.0 180.0) (0.0 0.0 1.0)) 2000.0) (`KismetMathLibrary.MakeRotator` 0.0 0.0 (`KismetMathLibrary.RandomFloatInRange` -180.0 180.0))))))
  (bind _returnvalue (`|SpawnActorFromClass` "/Game/NWV/Vehicle/Blueprint/PRT_NWheelVehicle.PRT_NWheelVehicle_C" (`local.Tr`) "Undefined" "MultiplyWithRoot" null null))
  (`/Engine/EditorBlueprintResources/StandardMacros.IsValid` _returnvalue
    (:`Is Valid`
      (`/Game/NWV/Vehicle/Blueprint/PRT_NWheelVehicle.LoadCar` _returnvalue (`self.Car Config`))
      (`Controller.Possess` (`self.PlayerController`) _returnvalue)
      (`Widget.RemoveFromParent` (`self.WidgetCarShare`))
      (set `PlayerController.bShowMouseCursor` false _playercontroller)
      (`WidgetBlueprintLibrary.SetInputMode_GameOnly` _playercontroller))))

(fn `UserConstructionScript`)