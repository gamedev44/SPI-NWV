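; BP_DummyCar is a dummy vehicle that assembles a car's visual appearance from a car config.
; LoadConfig sets the chassis mesh, destroys previously built wheel components, then rebuilds wheels from the axle data.
; Each wheel gets a hub scene component carrying position, camber and caster, with a collision-free mesh attached.
; The wheel index mirrors lateral offset, camber and mesh yaw, supporting up to two wheels per axle.
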(fn `AddWheels`
  (params (AxleConfig :type "Array of /Game/NWV/Vehicle/CustomType/Config/AxleConfig Structure"))
  (locals (index :type Integer))
  (bind _index (`local.index`))
  (for _array_element AxleConfig
    (bind (_numberofwheels _tracetype _tracesphereradius _drivetype _finalgearratio _differentialconfig _geometryconfig _wheelconfig) (break `/Game/NWV/Vehicle/CustomType/Config/AxleConfig` _array_element))
    (for _index_2 (range _numberofwheels)
      (set `local.index` _index_2)
      (bind (_wheelrefposition _toein _camber _caster) (break `/Game/NWV/Vehicle/CustomType/Config/GeometryConfig` _geometryconfig))
      (bind _returnvalue (`AddComponent|NODE_AddSceneComponent-0` :`RelativeTransform` (`KismetMathLibrary.MakeTransform` (`KismetMathLibrary.MakeVector` (.x _wheelrefposition) (* (.y _wheelrefposition) (select `int` _index :`0` -1.0 :`1` 1.0)) (.z _wheelrefposition)) (`KismetMathLibrary.MakeRotator` (* _camber (select `int` _index :`0` -1.0 :`1` 1.0)) _caster))))
      (`KismetArrayLibrary.Array_Add` (`self.WheelHub`) _returnvalue)
      (bind _returnvalue_2 (`AddComponent|NODE_AddStaticMeshComponent-0` :`RelativeTransform` (`KismetMathLibrary.MakeTransform` (0.0 0.0 0.0) (`KismetMathLibrary.MakeRotator` 0.0 0.0 (select `int` (`local.index`) :`0` 180.0 :`1` 0.0)))))
      (`KismetArrayLibrary.Array_Add` (`self.Wheels`) _returnvalue_2)
      (`StaticMeshComponent.SetStaticMesh` _returnvalue_2 (`.WheelMesh_18_6E9ABB70432816EB654141993570BB24` (break `/Game/NWV/Vehicle/CustomType/Config/WheelConfig` _wheelconfig)))
      (`PrimitiveComponent.SetCollisionEnabled` _returnvalue_2 "NoCollision")
      (`SceneComponent.K2_AttachToComponent` _returnvalue_2 _returnvalue "None" "KeepRelative" "KeepRelative" "KeepRelative" true))))

(fn `DestroyComponents`
  (for _array_element (`self.Wheels`)
    (`/Engine/EditorBlueprintResources/StandardMacros.IsValid` _array_element
      (:`Is Valid`
        (`ActorComponent.K2_DestroyComponent` _array_element))))
  (for _array_element_2 (`self.WheelHub`)
    (`/Engine/EditorBlueprintResources/StandardMacros.IsValid` _array_element_2
      (:`Is Valid`
        (`ActorComponent.K2_DestroyComponent` _array_element_2))))
  (`KismetArrayLibrary.Array_Clear` (`self.WheelHub`))
  (`KismetArrayLibrary.Array_Clear` (`self.Wheels`)))

(fn `Load Config`
  (params (CarConfig :type "/Game/NWV/Vehicle/CustomType/Config/CarConfig Structure"))
  (bind (_axle _mass _engine _clutch _gearbox _transmission _brakes _steering _carmesh) (break `/Game/NWV/Vehicle/CustomType/Config/CarConfig` CarConfig))
  (`StaticMeshComponent.SetStaticMesh` (`self.Body`) (`.Chassis_7_F941D1744CAE39EBD097ACBA1023184B` (break `/Game/NWV/Vehicle/CustomType/Config/CarMesh` _carmesh)))
  (`self.DestroyComponents`)
  (`self.AddWheels` _axle))

(fn `UserConstructionScript`)