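; Gearbox component for a vehicle drivetrain that converts torque toward the wheels and velocity and inertia back to the engine using the active gear ratio.
; Shifts drop to neutral until a custom timer, ticked by Update, applies the next gear.
; Auto-shift upshifts by speed and downshifts by RPM, using per-gear thresholds from UpdateShiftSpeed.
; Auto-reverse toggles reverse/first near standstill from brake/throttle input, flagging a pedal swap.
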(fn `AutoGearShift`
  (bind _gearindex (`self.GearIndex`))
  (bind _gearindex_2 (`self.GearIndex`))
  (if (> (- (`KismetSystemLibrary.GetGameTimeInSeconds`) (`self.LastAutoGearShiftTime`)) 0.5)
    (if (`self.SwapThrottleBrake`)
      (if (and (> (`self.EngineRPM`) 1000.0) (!= (`self.GearIndex`) -1))
        ;[1 1 1] set R gear
        (`self.ShiftGearByIndex` -1)
        (set `self.LastAutoGearShiftTime` (`KismetSystemLibrary.GetGameTimeInSeconds`) :!label _label))
      (elif (and (>= (`self.CarForwardSpeedMPS`) (`|GetArrayItem` (`self.UpShiftSpeedMPS`) (`KismetMathLibrary.Max` _gearindex_2 1))) (< _gearindex_2 (`KismetArrayLibrary.Array_LastIndex` (`self.GearRatioArray`))))
        (`self.ShiftGearUp`)
        (goto _label)
        (elif (and (<= (`self.EngineRPM`) (`|GetArrayItem` (`self.ShiftDownRPMArray`) (`KismetMathLibrary.Max` _gearindex 1))) (> _gearindex 1))
          (`self.ShiftGearDown`)
          (goto _label))))))

(fn `AutoReverse`
  (bind _gearindex (`self.GetGearIndex`))
  (bind _returnvalue (`KismetMathLibrary.NearlyEqual_FloatFloat` (`KismetMathLibrary.Abs` (`self.CarForwardSpeedMPS`)) 0.0 2.0))
  ;[1 1 1] check if enough time has passed since the last function call
  (if (> (- (`KismetSystemLibrary.GetGameTimeInSeconds`) (`self.LastAutoReverseTime`)) 0.5)
    (if (and (> (`self.BrakeInput`) 0.0) _returnvalue (!= _gearindex -1))
      ;[1 1 1] swap throttle brake input
      (set `self.SwapThrottleBrake` true)
      ;[1 1 1] Set Reverse
      (set `self.NextGearIndex` -1)
      (`self.Processing` (`self.NextGearIndex`) :!label _label)
      (set `self.LastAutoReverseTime` (`KismetSystemLibrary.GetGameTimeInSeconds`))
      (elif (and (> (`self.ThrottleInput`) 0.0) _returnvalue (!= _gearindex 1))
        (set `self.SwapThrottleBrake` false)
        ;[1 1 1] Set 1st Gear
        (set `self.NextGearIndex` 1)
        (goto _label)))))

(fn `Change Gear Callback`
  (if (== (`self.NextGearIndex`) -1)
    (set `self.GearRatio` (* (`KismetMathLibrary.Abs` (`self.ReverseGearRatio`)) -1.0))
    (set `self.IsReverseGear` true)
    (else
      (set `self.GearRatio` (`|GetArrayItem` (`self.GearRatioArray`) (`self.NextGearIndex`)))
      (set `self.IsReverseGear` false)))
  (bind _output_get (set `self.GearIndex` (`self.NextGearIndex`)))
  (set `self.IsGearChangeInProgress` false)
  (`KismetSystemLibrary.PrintString` (`KismetStringLibrary.Concat_StrStr` "Gearbox::  " (`KismetStringLibrary.Conv_IntToString` _output_get) " Gear") false false (struct :`G` 0.66 :`B` 1.0 :`A` 1.0) 0.0))

(fn `GetAutoGearShiftArrays`
  (returns (UpShiftSpeedMPS :type "Array of Float (double-precision)") (DownShiftSpeedMPS :type "Array of Float (double-precision)") (MaxSpeedOnGear :type "Array of Float (double-precision)"))
  (return (`self.UpShiftSpeedMPS`) (`self.DownShiftSpeedMPS`) (`self.MaxSpeedOnGear`)))

(fn `GetGearChangeInProgress`
  (returns (IsGearChangeInProgress :type Boolean))
  (return (`self.IsGearChangeInProgress`)))

(fn `GetGearIndex`
  (returns (GearIndex :type Integer))
  (return (`self.GearIndex`)))

(fn `GetGearRatio`
  (returns (GearRatio :type "Float (double-precision)"))
  (return (`self.GearRatio`)))

(fn `GetIsReverseGear`
  (returns (Value :type Boolean))
  (return (`self.IsReverseGear`)))

(fn `GetSwap`
  (returns (Value :type Boolean))
  (return (`self.SwapThrottleBrake`)))

(fn `Initialize`
  (bind _gearindex (`self.GearIndex`))
  (set `self.GearRatio` (select `bool` (== _gearindex -1) :`false` (`|GetArrayItem` (`self.GearRatioArray`) _gearindex) :`true` (`self.ReverseGearRatio`))))

(fn `Processing`
  (params (IndexToTest :type Integer))
  (if (`self.IsGearChangeInProgress`)
    _
    (elif (`KismetArrayLibrary.Array_IsValidIndex` (`self.GearRatioArray`) IndexToTest)
      (set `self.IsGearChangeInProgress` true :!label _label)
      (set `self.NextGearIndex` IndexToTest)
      (`self.SetNeutralGear`)
      ;[1 1 1] activate custom timer
      (`self.TimerStart`)
      (elif (== IndexToTest -1)
        (goto _label)))))

(fn `RPMToRad`
  (params (RPM :type "Float (double-precision)"))
  (returns (RadS :type "Float (double-precision)"))
  (return (/ (* RPM (`KismetMathLibrary.GetPI`)) 30.0)))

(fn `SetAutoReverse`
  (params (IsAutoReverse :type Boolean))
  (set `self.IsAutoReverse` IsAutoReverse))

(fn `SetAutoShift`
  (params (IsAutoShift :type Boolean))
  (set `self.IsAutoShift` IsAutoShift))

(fn `SetConfig`
  (params (GearboxConfig :type "/Game/NWV/Vehicle/CustomType/Config/GearboxConfig Structure (by ref)"))
  (bind (_gearratio _reversegearratio _shifttime) (break `/Game/NWV/Vehicle/CustomType/Config/GearboxConfig` GearboxConfig))
  (set `self.GearRatioArray` _gearratio)
  (set `self.ReverseGearRatio` _reversegearratio)
  (set `self.GearChangeTime` _shifttime))

(fn `SetNeutralGear`
  (set `self.GearRatio` 0.0))

(fn `ShiftGearByIndex`
  (params (Index :type Integer))
  (`self.Processing` Index))

(fn `ShiftGearDown`
  (`self.Processing` (- (`self.GearIndex`) 1)))

(fn `ShiftGearUp`
  (`self.Processing` (+ (`self.GearIndex`) 1)))

(fn `TimerStart`
  (set `self.ElapsedTime` 0.0)
  (set `self.IsTimerEnabled` true))

(fn `TimerStop`
  (set `self.ElapsedTime` 0.0)
  (set `self.IsTimerEnabled` false))

(fn `TimerUpdate`
  (if (`self.IsTimerEnabled`)
    (set `self.ElapsedTime` (+ (`self.ElapsedTime`) (`self.DeltaTime`))))
  (if (>= (`self.ElapsedTime`) (`self.GearChangeTime`))
    (`self.TimerStop`)
    (`self.Change Gear Callback`)))

(fn `ToEngine`
  (params (VelocityIn :type "Float (double-precision)") (InertiaIn :type "Float (double-precision)"))
  (returns (VelocityOut :type "Float (double-precision)") (InertiaOut :type "Float (double-precision)"))
  (bind _gearratio (`self.GearRatio`))
  (return (* VelocityIn _gearratio) (`KismetMathLibrary.SafeDivide` InertiaIn (* _gearratio _gearratio))))

(fn `ToWheels`
  (params (TorqueIn :type "Float (double-precision)"))
  (returns (TorqueOut :type "Float (double-precision)"))
  (return (* TorqueIn (`self.GearRatio`))))

(fn `Update`
  (params (ThrottleInput :type "Float (double-precision)") (BrakeInput :type "Float (double-precision)") (CarForwardSpeedMPS :type "Float (double-precision)") (EngineRPM :type "Float (double-precision)") (DeltaTime :type "Float (double-precision)"))
  (set `self.ThrottleInput` ThrottleInput)
  (set `self.BrakeInput` BrakeInput)
  (set `self.CarForwardSpeedMPS` CarForwardSpeedMPS)
  (set `self.EngineRPM` EngineRPM)
  (set `self.DeltaTime` DeltaTime)
  (`self.TimerUpdate`)
  (if (`self.IsAutoReverse`)
    (`self.AutoReverse`))
  (if (`self.IsAutoShift`)
    (`self.AutoGearShift`)))

(fn `UpdateShiftSpeed`
  (params (EngineMaxRPM :type "Float (double-precision)") (FinalGearRatio :type "Float (double-precision)") (WheelRadiusM :type "Float (double-precision)"))
  (locals (Index :type Integer))
  (bind _enginemaxrpm (`self.EngineMaxRPM`))
  (bind _returnvalue (* _enginemaxrpm (select `int` (`local.Index`) :`0` 0.4 :`1` 0.4 :`2` 0.4 :`3` 0.42 :`4` 0.5 :`5` 0.53 :`6` 0.57 :`7` 0.6 :`8` 0.6)))
  (`KismetArrayLibrary.Array_Clear` (`self.UpShiftSpeedMPS`))
  (`KismetArrayLibrary.Array_Clear` (`self.DownShiftSpeedMPS`))
  (`KismetArrayLibrary.Array_Clear` (`self.MaxSpeedOnGear`))
  (`KismetArrayLibrary.Array_Clear` (`self.ShiftDownRPMArray`))
  (`KismetArrayLibrary.Array_Clear` (`self.ArrayGearCheck`))
  (set `self.EngineMaxRPM` EngineMaxRPM)
  (for (_array_element _array_index) (`self.GearRatioArray`)
    (set `local.Index` _array_index)
    (bind _returnvalue_2 (* _array_element FinalGearRatio))
    ;[1 1 1] максимальная скорость в м\с для каждой передачи
    (`KismetArrayLibrary.Array_Add` (`self.MaxSpeedOnGear`) (* (`KismetMathLibrary.SafeDivide` (`self.RPMToRad` EngineMaxRPM) _returnvalue_2) WheelRadiusM))
    (`KismetArrayLibrary.Array_Add` (`self.UpShiftSpeedMPS`) (* (`KismetMathLibrary.SafeDivide` (`self.RPMToRad` (* _enginemaxrpm (select `int` (`local.Index`) :`0` 0.8 :`1` 0.7 :`2` 0.72 :`3` 0.73 :`4` 0.75 :`5` 0.77 :`6` 0.85 :`7` 0.9 :`8` 0.95))) _returnvalue_2) WheelRadiusM))
    (`KismetArrayLibrary.Array_Add` (`self.DownShiftSpeedMPS`) (* (`KismetMathLibrary.SafeDivide` (`self.RPMToRad` _returnvalue) _returnvalue_2) WheelRadiusM))
    (`KismetArrayLibrary.Array_Add` (`self.ShiftDownRPMArray`) _returnvalue)
    ;[1 1 1] for debug purposes
    (`KismetArrayLibrary.Array_Add` (`self.ArrayGearCheck`) _array_element)))